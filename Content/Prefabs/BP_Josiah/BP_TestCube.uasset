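; BP_TestCube is a test cube that reacts to magic missile hits and a levitation glow toggle.
; On a hit from a BP_MagicMissile, it applies a large impulse to the cube along the missile sphere's forward vector for knockback.
; Levitate flips a Floating flag and adds or clears an overlay material as a glow, without moving the cube itself.
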(event `self.ReceiveHit`
  (params (MyComp :type "PrimitiveComponent Object Reference") (Other :type "Actor Object Reference") (OtherComp :type "PrimitiveComponent Object Reference") (bSelfMoved :type Boolean) (HitLocation :type "Vector Structure") (HitNormal :type "Vector Structure") (NormalImpulse :type "Vector Structure") (Hit :type "HitResult Structure (by ref)"))
  ; Knockback when hit by magic missile
  (bind _asbp_magic_missile (cast `/Game/Prefabs/BP_Josiah/BP_MagicMissile` Other))
  (`PrimitiveComponent.AddImpulse` (`self.Cube`) (* (`SceneComponent.GetForwardVector` (`/Game/Prefabs/BP_Josiah/BP_MagicMissile.Sphere` _asbp_magic_missile)) (300000.0 300000.0 300000.0)) "None" false))

(event `/Game/Input/Interface/BPI_Levitate.Levitate`
  (bind _cube (`self.Cube`))
  ; Flipflop for glow effect
  (if (`self.Floating`)
    (`MeshComponent.SetOverlayMaterial` _cube null)
    (set `self.Floating` false)
    (else
      (`MeshComponent.SetOverlayMaterial` _cube "/Game/Materials/Mat_Overlay.Mat_Overlay")
      (set `self.Floating` true))))

(fn `UserConstructionScript`)