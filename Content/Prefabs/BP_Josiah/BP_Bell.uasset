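; BP_Bell is a physics bell that rings through its BP_Socket when triggered while mounted, and otherwise prints "Thunk".
; It starts attached to any preassigned socket, and magic missile hits knock it away only while unsocketed.
; Levitate detaches it from its socket with physics enabled and toggles a floating glow overlay.
; Toggling floating off snaps the bell onto an overlapping socket's attach point and notifies that socket.
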(event `self.Trigger`
  ; Rings if attached to socket
  (bind _bellsocket (`self.BellSocket`)
    (:`then`
      (`/Game/Prefabs/BP_Josiah/BP_Socket.Ring` _bellsocket))
    (:`else`
      (`KismetSystemLibrary.PrintString` "Thunk"))))

(event `self.ReceiveHit`
  (params (MyComp :type "PrimitiveComponent Object Reference") (Other :type "Actor Object Reference") (OtherComp :type "PrimitiveComponent Object Reference") (bSelfMoved :type Boolean) (HitLocation :type "Vector Structure") (HitNormal :type "Vector Structure") (NormalImpulse :type "Vector Structure") (Hit :type "HitResult Structure (by ref)"))
  ; Knockback when hit by magic missile
  (bind _asbp_magic_missile (cast `/Game/Prefabs/BP_Josiah/BP_MagicMissile` Other))
  (`self.BellSocket`
    (:`then`)
    (:`else`
      (`PrimitiveComponent.AddImpulse` (`self.Bell`) (* (`SceneComponent.GetForwardVector` (`/Game/Prefabs/BP_Josiah/BP_MagicMissile.Sphere` _asbp_magic_missile)) (300000.0 300000.0 300000.0)) "None" false))))

(event `self.Levitate`
  (bind _bell (`self.Bell`))
  (bind _bell_2 (`self.Bell`))
  ; Removes from socket if attached
  (bind _bellsocket (`self.BellSocket`)
    (:`then`
      (`/Game/Prefabs/BP_Josiah/BP_Socket.RemoveBell` _bellsocket)
      (`SceneComponent.K2_DetachFromComponent` _bell_2 "KeepRelative" "KeepRelative" "KeepWorld" true)
      (`PrimitiveComponent.SetSimulatePhysics` _bell_2 true)
      (set `self.BellSocket` null))
    (:`else`
      _))
  ; Flipflop for glow effect
  (if (`self.Floating`)
    (`MeshComponent.SetOverlayMaterial` _bell null)
    (set `self.Floating` false)
    ; Checks for nearby sockets and attaches
    (for _array_element (`self.GetOverlappingActors` "/Game/Prefabs/BP_Josiah/BP_Socket.BP_Socket_C")
      (bind _asbp_socket (cast `/Game/Prefabs/BP_Josiah/BP_Socket` _array_element))
      (bind _output_get (set `self.BellSocket` _asbp_socket))
      (`SceneComponent.K2_AttachToComponent` (`self.Bell`) (`/Game/Prefabs/BP_Josiah/BP_Socket.AttachPoint` _asbp_socket) "None" "SnapToTarget" "SnapToTarget" "KeepWorld" true)
      (`/Game/Prefabs/BP_Josiah/BP_Socket.AttachBell` _output_get))
    (else
      (`MeshComponent.SetOverlayMaterial` _bell "/Game/Materials/Mat_Overlay.Mat_Overlay")
      (set `self.Floating` true))))

(event `self.ReceiveBeginPlay`
  ; Attaches if default
  (bind _bellsocket (`self.BellSocket`)
    (:`then`
      (`SceneComponent.K2_AttachToComponent` (`self.Bell`) (`/Game/Prefabs/BP_Josiah/BP_Socket.AttachPoint` _bellsocket) "None" "SnapToTarget" "SnapToTarget" "KeepWorld" true)
      (`/Game/Prefabs/BP_Josiah/BP_Socket.AttachBell` _bellsocket))
    (:`else`)))

(fn `UserConstructionScript`)