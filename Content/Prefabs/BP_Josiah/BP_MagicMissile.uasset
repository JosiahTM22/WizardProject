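; BP_MagicMissile is a magic missile projectile that fires triggers on objects it hits.
; It uses a ProjectileMovement component, a collision Sphere and a Niagara effect.
; On hit, it sends TriggerMessage to actors implementing BPI_Trigger, restarts Niagara, disables collision on the Niagara component and destroys itself shortly after.
; BeginPlay also activates Niagara and destroys the actor after 0.5 seconds, despite its comment saying 3 seconds.
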(event `self.ReceiveBeginPlay`
  ; Destroy the projectile after 3 seconds
  (`ActorComponent.Activate` (`self.Niagara`) false)
  (`KismetSystemLibrary.Delay` 0.5)
  (`self.K2_DestroyActor`))

(event `self.Sphere.OnComponentHit`
  (params (HitComponent :type "PrimitiveComponent Object Reference") (OtherActor :type "Actor Object Reference") (OtherComp :type "PrimitiveComponent Object Reference") (NormalImpulse :type "Vector Structure") (Hit :type "HitResult Structure (by ref)"))
  (bind _niagara (`self.Niagara`))
  ; Magic Missile Trigger - Checks object collided with, calls trigger if it has the trigger interface, destroys the projectile.
  (if (`KismetSystemLibrary.DoesImplementInterface` OtherActor "/Game/Input/Interface/BPI_Trigger.BPI_Trigger_C")
    (message `/Game/Input/Interface/BPI_Trigger.Trigger` OtherActor))
  (`ActorComponent.Activate` _niagara false)
  (`PrimitiveComponent.SetCollisionEnabled` _niagara "NoCollision")
  (`KismetSystemLibrary.Delay` 0.5)
  (`self.K2_DestroyActor`))

(event `self.ProjectileMovement.OnComponentActivated`
  (params (Component :type "ActorComponent Object Reference") (bReset :type Boolean)))

(fn `UserConstructionScript`)