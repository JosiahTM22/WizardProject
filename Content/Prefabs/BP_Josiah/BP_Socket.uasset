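; BP_Socket is a bell socket that works as a switch for a linked door.
; Ring, noted as firing when an attached bell is hit by a projectile, sends BellValue to DoorToActivate once and shows a point light.
; RemoveBell re-enables Box overlap events and, if triggered, deactivates the door switch and hides the light.
; AttachBell disables those overlap events while the socket is occupied.
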(event `Ring`
  ; Plays when a bell is attached and hit by a projectile
  (`KismetSystemLibrary.PrintString` "Ring")
  (if (not (`self.Triggered`))
    (bind _doortoactivate (`self.DoorToActivate`)
      (:`then`
        (`/Game/Prefabs/BP_Josiah/BP_Door.SwitchActivated` _doortoactivate (`self.BellValue`))
        (set `self.Triggered` true)
        (`SceneComponent.SetVisibility` (`self.PointLight`) true false))
      (:`else`))))

(event `RemoveBell`
  ; Triggers when the bell is taken off
  (`KismetSystemLibrary.PrintString` "Click")
  (set `PrimitiveComponent.bGenerateOverlapEvents` true (`self.Box`))
  (if (`self.Triggered`)
    (bind _doortoactivate (`self.DoorToActivate`)
      (:`then`
        (`/Game/Prefabs/BP_Josiah/BP_Door.SwitchDeactivated` _doortoactivate (`self.BellValue`))
        (set `self.Triggered` false)
        (`SceneComponent.SetVisibility` (`self.PointLight`) false false))
      (:`else`))))

(event `AttachBell`
  ; Triggers when the bell is attached
  (set `PrimitiveComponent.bGenerateOverlapEvents` false (`self.Box`)))

(fn `UserConstructionScript`)