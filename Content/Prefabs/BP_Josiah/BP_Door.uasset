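; BP_Door is a sliding double door for switch puzzles, driven by either a count of active switches or an ordered sequence.
; Positive switch numbers must match the Order array, with mistakes or deactivations resetting progress and completion opening it permanently.
; Other signals adjust an active count against a threshold, closing the door again unless OneTimeOpen latches it.
; A timeline plays forward or reverse to slide both halves oppositely, with fading movement audio.
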(event `self.ReceiveBeginPlay`
  ; Sets Puzzle Length
  (set `self.OrderNeeded` (`KismetArrayLibrary.Array_Length` (`self.Order`))))

(event `SwitchActivated`
  (params (OpenNum :type Integer))
  (bind _sc_movedoor (`self.SC_MoveDoor`))
  (bind _sc_movedoor_2 (`self.SC_MoveDoor`))
  (bind _doorl (`self.DoorL`))
  (bind _doorr (`self.DoorR`))
  (bind (_relativelocation_x _relativelocation_y _relativelocation_z) (`KismetMathLibrary.BreakVector` (`SceneComponent.RelativeLocation` _doorl)))
  (bind (_relativelocation_x_2 _relativelocation_y_2 _relativelocation_z_2) (`KismetMathLibrary.BreakVector` (`SceneComponent.RelativeLocation` _doorr)))
  (bind _returnvalue (== (`|GetArrayItem` (`self.Order`) (`self.OrderCurrent`)) (`self.Open Num`)))
  ; Checks if the signal is normal or ordered
  (bind _output_get (set `self.Open Num` OpenNum))
  (if (> _output_get 0)
    ; Check Order
    (if _returnvalue
      (bind _output_get_2 (set `self.OrderCurrent` (+ (`self.OrderCurrent`) 1) :!label _label))
      (if (== (`self.OrderNeeded`) _output_get_2)
        ; Checks if the door opens permanently
        (set `self.Opened` true :!label _label_2)
        ; Door Audio
        (bind _doorsfx (`self.DoorSFX` :!label _label_3)
          (:`then`
            (`AudioComponent.Stop` _doorsfx))
          (:`else`
            _))
        (`AudioComponent.FadeIn` _sc_movedoor_2 0.1 1.0 0.0 "Linear")
        (set `self.DoorSFX` _sc_movedoor_2)
        ; Open/Close animation
        (bind (_direction _doorposition) (`Timeline|DoorActivation` :!label _label_4)
          (:`Update`
            (`SceneComponent.K2_SetRelativeLocation` _doorr (`KismetMathLibrary.MakeVector` _relativelocation_x_2 _doorposition _relativelocation_z_2) false false)
            (`SceneComponent.K2_SetRelativeLocation` _doorl (`KismetMathLibrary.MakeVector` _relativelocation_x (* _doorposition -1.0) _relativelocation_z) false false))
          (:`Finished`
            (`AudioComponent.FadeOut` (`self.DoorSFX`) 0.2 0.0 "Linear"))))
      (else
        (set `self.OrderCurrent` 0)
        (if _returnvalue
          (goto _label))))
    (else
      ; Opens and closes door based on the number of activated switches
      (`/Engine/EditorBlueprintResources/StandardMacros.IncrementInt` (`self.SwitchesActive`)
        (:`  `
          (if (`self.Opened`) :!label _label_5
            _
            (elif (>= (`self.SwitchesActive`) (`self.SwitchesNeeded`))
              (if (`self.OneTimeOpen`)
                (goto _label_2)
                (else
                  (goto _label_3)))
              (else
                (bind _doorsfx_2 (`self.DoorSFX`)
                  (:`then`
                    (`AudioComponent.Stop` _doorsfx_2))
                  (:`else`
                    _))
                (`AudioComponent.FadeIn` _sc_movedoor 0.1 1.0 0.0 "Linear")
                (set `self.DoorSFX` _sc_movedoor)
                (goto _label_4 :!via `Reverse`)))))))))

(event `SwitchDeactivated`
  (params (CloseNum :type Integer))
  ; Checks if the signal is normal or ordered
  (if (> CloseNum 0)
    (set `self.OrderCurrent` 0)
    (else
      ; Opens and closes door based on the number of activated switches
      (`/Engine/EditorBlueprintResources/StandardMacros.DecrementInt` (`self.SwitchesActive`)
        (:`  `
          (goto _label_5))))))

(fn `UserConstructionScript`)