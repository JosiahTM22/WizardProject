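; BP_BellPuzzle is a bell-ordering puzzle manager that checks the order in which bells are triggered.
; On BeginPlay it finds every BP_Bell_old actor and assigns itself as their PuzzleRef.
; RegisterBellInput compares each input index to CorrectSequence at CurrentStep, advancing on a match and resetting to zero on a mistake.
; Completing the sequence only prints a "Door Opened" message; no door logic exists here.
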(event `self.ReceiveBeginPlay`
  (bind _outactors (`GameplayStatics.GetAllActorsOfClass` "/Game/Prefabs/BP_Yeonji/BP_Bell_old.BP_Bell_old_C"))
  (for _array_element _outactors
    (set `/Game/Prefabs/BP_Yeonji/BP_Bell_old.PuzzleRef` self _array_element)))

(fn `RegisterBellInput`
  (params (InputIndex :type Integer))
  (if (== InputIndex (`|GetArrayItem` (`self.CorrectSequence`) (`self.CurrentStep`)))
    (set `self.CurrentStep` (+ (`self.CurrentStep`) 1))
    (if (== (`self.CurrentStep`) (`KismetArrayLibrary.Array_Length` (`self.CorrectSequence`)))
      (`KismetSystemLibrary.PrintString` "Door Opened"))
    (else
      (set `self.CurrentStep` 0)
      (`KismetSystemLibrary.PrintString` "Wrong order"))))

(fn `UserConstructionScript`)