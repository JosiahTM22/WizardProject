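; BP_Bell is one bell in a bell puzzle, rung when a BP_MagicMissile overlaps its trigger box.
; A valid hit swings the mesh with a timeline that offsets roll from the rotation cached at BeginPlay and plays the bell sound at the actor's location.
; It then passes its BellIndex to the referenced puzzle's RegisterBellInput, and only prints an error if that reference is invalid.
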(event `self.ReceiveBeginPlay`
  ; Event Begin Play
  (set `self.InitialBellRotation` (`SceneComponent.RelativeRotation` (`self.BellMesh`))))

(event `self.TriggerBox.OnComponentBeginOverlap`
  (params (OverlappedComponent :type "PrimitiveComponent Object Reference") (OtherActor :type "Actor Object Reference") (OtherComp :type "PrimitiveComponent Object Reference") (OtherBodyIndex :type Integer) (bFromSweep :type Boolean) (SweepResult :type "HitResult Structure (by ref)"))
  ; Begin Overlap
  (cast `/Game/Prefabs/BP_Josiah/BP_MagicMissile` OtherActor)
  (`/Engine/EditorBlueprintResources/StandardMacros.IsValid` (`self.PuzzleRef`)
    (:`Is Valid`
      (`|ExecutionSequence`
        (:`then_0`
          ;; Play Animation
          (bind (_direction _swingalpha) (`Timeline|TL_BellSwing` :!via `PlayFromStart`)
            (:`Update`
              (`SceneComponent.K2_SetRelativeRotation` (`self.BellMesh`) (`KismetMathLibrary.MakeRotator` (+ (.roll (`self.InitialBellRotation`)) (* _swingalpha (`self.SwingAngle`))) (.pitch (`self.InitialBellRotation`)) (.yaw (`self.InitialBellRotation`))) false false))))
        (:`then_1`
          ;; Play Note
          (`GameplayStatics.PlaySoundAtLocation` (`self.BellSound`) (`self.K2_GetActorLocation`) (struct) 1.0 1.0 0.0 null null null null))
        (:`then_2`
          ;; Count List
          (`/Game/Prefabs/BP_Yeonji/BP_BellPuzzle.RegisterBellInput` (`self.PuzzleRef`) (`self.BellIndex`)))))
    (:`Is Not Valid`
      (`KismetSystemLibrary.PrintString` "PuzzleRef invalid"))))

(fn `UserConstructionScript`)