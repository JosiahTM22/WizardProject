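; BP_SoundTrigger is a trigger volume actor that plays a repeating 2D bell sound while something overlaps it.
; Overlap begin on TriggerBox sets an IsPlaying flag and starts PlayBellLoop, which plays the sound, waits on a Delay, then calls itself again while the flag holds.
; Overlap end clears the flag, and neither overlap event filters which actor triggered it.
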(event `self.TriggerBox.OnComponentBeginOverlap`
  (params (OverlappedComponent :type "PrimitiveComponent Object Reference") (OtherActor :type "Actor Object Reference") (OtherComp :type "PrimitiveComponent Object Reference") (OtherBodyIndex :type Integer) (bFromSweep :type Boolean) (SweepResult :type "HitResult Structure (by ref)"))
  (if (not (`self.IsPlaying`))
    (set `self.IsPlaying` true)
    (`self.PlayBellLoop`)))

(event `PlayBellLoop`
  (`GameplayStatics.PlaySound2D` null 1.0 1.0 0.0 null null)
  (`KismetSystemLibrary.Delay` 5.0)
  (if (`self.IsPlaying`)
    (`self.PlayBellLoop`)))

(event `self.TriggerBox.OnComponentEndOverlap`
  (params (OverlappedComponent :type "PrimitiveComponent Object Reference") (OtherActor :type "Actor Object Reference") (OtherComp :type "PrimitiveComponent Object Reference") (OtherBodyIndex :type Integer))
  (set `self.IsPlaying` false))

(fn `UserConstructionScript`)