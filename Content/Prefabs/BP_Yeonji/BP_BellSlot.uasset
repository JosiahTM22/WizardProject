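; BP_BellSlot is a puzzle slot that checks whether a BP_Bell with a matching index sits inside its trigger.
; It compares SlotIndex to BellIndex at BeginPlay and on begin overlap, setting the bell's IsPlacedCorrectly on a match, and end overlap clears that flag.
; AssignedSlot points to this slot after a matching begin overlap or any end overlap, but is cleared by a BeginPlay match or mismatched begin overlap.
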(event `self.ReceiveBeginPlay`
  ; Event BeginPlay - Check if bell overlaps with bellSlot when the game starts
  (for _array_element (`PrimitiveComponent.GetOverlappingActors` (`self.SlotTrigger`) null)
    (bind _asbp_bell (cast `/Game/Prefabs/BP_Yeonji/BP_Bell` _array_element))
    (if (== (`self.SlotIndex`) (`/Game/Prefabs/BP_Yeonji/BP_Bell.BellIndex` _asbp_bell))
      (set `/Game/Prefabs/BP_Yeonji/BP_Bell.IsPlacedCorrectly` true _asbp_bell)
      (set `/Game/Prefabs/BP_Yeonji/BP_Bell.AssignedSlot` null _asbp_bell)
      (else
        (`KismetSystemLibrary.PrintString` "Begin Play Wrong SLot")))))

(event `self.SlotTrigger.OnComponentBeginOverlap`
  (params (OverlappedComponent :type "PrimitiveComponent Object Reference") (OtherActor :type "Actor Object Reference") (OtherComp :type "PrimitiveComponent Object Reference") (OtherBodyIndex :type Integer) (bFromSweep :type Boolean) (SweepResult :type "HitResult Structure (by ref)"))
  ; Begin Overlap -  Check if bell overlaps with slot and index matches slot index
  (bind _asbp_bell (cast `/Game/Prefabs/BP_Yeonji/BP_Bell` OtherActor))
  (if (== (`self.SlotIndex`) (`/Game/Prefabs/BP_Yeonji/BP_Bell.BellIndex` _asbp_bell))
    (`KismetSystemLibrary.PrintString` "Correct Slot")
    (set `/Game/Prefabs/BP_Yeonji/BP_Bell.IsPlacedCorrectly` true _asbp_bell)
    (set `/Game/Prefabs/BP_Yeonji/BP_Bell.AssignedSlot` self _asbp_bell)
    (else
      (`KismetSystemLibrary.PrintString` "Wrong Slot")
      (set `/Game/Prefabs/BP_Yeonji/BP_Bell.IsPlacedCorrectly` false _asbp_bell)
      (set `/Game/Prefabs/BP_Yeonji/BP_Bell.AssignedSlot` null _asbp_bell))))

(event `self.SlotTrigger.OnComponentEndOverlap`
  (params (OverlappedComponent :type "PrimitiveComponent Object Reference") (OtherActor :type "Actor Object Reference") (OtherComp :type "PrimitiveComponent Object Reference") (OtherBodyIndex :type Integer))
  ; End Overlap - Check if bell is no longer overlapping the slot
  (bind _asbp_bell (cast `/Game/Prefabs/BP_Yeonji/BP_Bell` OtherActor))
  (set `/Game/Prefabs/BP_Yeonji/BP_Bell.IsPlacedCorrectly` false _asbp_bell)
  (set `/Game/Prefabs/BP_Yeonji/BP_Bell.AssignedSlot` self _asbp_bell))

(fn `UserConstructionScript`)