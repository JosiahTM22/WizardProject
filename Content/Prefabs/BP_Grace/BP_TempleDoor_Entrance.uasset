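; BP_TempleDoor_Entrance is a temple entrance door that opens while enough switches are active and closes otherwise.
; SwitchActivated and SwitchDeactivated adjust a counter, then compare it to SwitchesNeeded to play or reverse the DoorActivation timeline.
; The timeline offsets the door's height from the world Z cached at BeginPlay, though it applies the result as a relative location.
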(event `self.ReceiveBeginPlay`
  (bind (_returnvalue_x _returnvalue_y _returnvalue_z) (`KismetMathLibrary.BreakVector` (`SceneComponent.K2_GetComponentLocation` (`self.Door`))))
  ; Finds the default height of the door
  (set `self.DoorZ` _returnvalue_z))

(event `SwitchActivated`
  ; Opens and closes door based on the number of activated switches
  (`/Engine/EditorBlueprintResources/StandardMacros.IncrementInt` (`self.SwitchesActive`)
    (:`  `
      (if (>= (`self.SwitchesActive`) (`self.SwitchesNeeded`)) :!label _label
        (bind (_direction _doorposition) (`Timeline|DoorActivation` :!label _label_2)
          (:`Update`
            (`SceneComponent.K2_SetRelativeLocation` (`self.Door`) (`KismetMathLibrary.MakeVector` 0.0 0.0 (+ (`self.DoorZ`) _doorposition)) false false)))
        (else
          (goto _label_2 :!via `Reverse`))))))

(event `SwitchDeactivated`
  ; Opens and closes door based on the number of activated switches
  (`/Engine/EditorBlueprintResources/StandardMacros.DecrementInt` (`self.SwitchesActive`)
    (:`  `
      (goto _label))))

(fn `UserConstructionScript`)