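; BP_Symbol is an actor that briefly reveals a hidden symbol and rings a bell sound when hit by a BP_MagicMissile.
; On hit, if the Visible flag is set, Ring adds an audio component picked by BellValue.
; SymbolType then selects one of six Niagara effects (butterfly, circle, dragon, moon, star, sun).
; Visible is cleared while the effect plays, blocking re-triggers until it deactivates five seconds later.
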(event `self.ReceiveHit`
  (params (MyComp :type "PrimitiveComponent Object Reference") (Other :type "Actor Object Reference") (OtherComp :type "PrimitiveComponent Object Reference") (bSelfMoved :type Boolean) (HitLocation :type "Vector Structure") (HitNormal :type "Vector Structure") (NormalImpulse :type "Vector Structure") (Hit :type "HitResult Structure (by ref)"))
  ; Hit with Magic Missile, reveals symbol.
  (bind _asbp_magic_missile (cast `/Game/Prefabs/BP_Josiah/BP_MagicMissile` Other))
  (if (`self.Visible`)
    (`self.Ring`)
    (switch `int` (`self.SymbolType`)
      (:`1`
        ; Determines what symbol is shown
        ;; Butterfly
        (bind _returnvalue (`AddComponent|NODE_AddNiagaraComponent-1`))
        (set `self.Visible` false)
        (`KismetSystemLibrary.Delay` 5.0)
        (`ActorComponent.Deactivate` _returnvalue)
        (set `self.Visible` true))
      (:`2`
        ;; Circle
        (bind _returnvalue_2 (`AddComponent|NODE_AddNiagaraComponent-2`))
        (set `self.Visible` false)
        (`KismetSystemLibrary.Delay` 5.0)
        (`ActorComponent.Deactivate` _returnvalue_2)
        (set `self.Visible` true))
      (:`3`
        ;; Dragon
        (bind _returnvalue_3 (`AddComponent|NODE_AddNiagaraComponent-3`))
        (set `self.Visible` false)
        (`KismetSystemLibrary.Delay` 5.0)
        (`ActorComponent.Deactivate` _returnvalue_3)
        (set `self.Visible` true))
      (:`4`
        ;; Moon
        (bind _returnvalue_4 (`AddComponent|NODE_AddNiagaraComponent-4`))
        (set `self.Visible` false)
        (`KismetSystemLibrary.Delay` 5.0)
        (`ActorComponent.Deactivate` _returnvalue_4)
        (set `self.Visible` true))
      (:`5`
        ;; Star
        (bind _returnvalue_5 (`AddComponent|NODE_AddNiagaraComponent-5`))
        (set `self.Visible` false)
        (`KismetSystemLibrary.Delay` 5.0)
        (`ActorComponent.Deactivate` _returnvalue_5)
        (set `self.Visible` true))
      (:`6`
        ;; Sun
        (bind _returnvalue_6 (`AddComponent|NODE_AddNiagaraComponent-6`))
        (set `self.Visible` false)
        (`KismetSystemLibrary.Delay` 5.0)
        (`ActorComponent.Deactivate` _returnvalue_6)
        (set `self.Visible` true)))))

(event `Ring`
  ; Plays when hit by projectile
  (switch `int` (`self.BellValue`)
    (:`1`
      (`AddComponent|NODE_AddAudioComponent-10`))
    (:`2`
      (`AddComponent|NODE_AddAudioComponent-11`))
    (:`3`
      (`AddComponent|NODE_AddAudioComponent-12`))
    (:`4`
      (`AddComponent|NODE_AddAudioComponent-14`))
    (:`5`
      (`AddComponent|NODE_AddAudioComponent-9`))
    (:`6`
      (`AddComponent|NODE_AddAudioComponent-15` :`bManualAttachment` true))
    (:`7`
      (`AddComponent|NODE_AddAudioComponent-13`))))

(fn `UserConstructionScript`)