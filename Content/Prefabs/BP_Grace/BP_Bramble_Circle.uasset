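; A burnable bramble circle actor that, once burned, removes its linked barrier and frees a referenced bell.
; BeginPlay creates and stores a dynamic material instance for each static mesh material.
; Burn destroys the barrier, disables mesh collision, fades in the burn sound and plays a timeline that drives each material's Dissolve parameter.
; When the timeline finishes, it calls FreeBell on the bell and destroys itself.
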(event `self.ReceiveBeginPlay`
  ; Dissolve VFX, dissolves each material on actor
  (for (_array_element _array_index) (`MeshComponent.GetMaterials` (`self.StaticMesh`))
    ;; Dissolves both materials
    (bind _returnvalue (`KismetMaterialLibrary.CreateDynamicMaterialInstance` _array_element))
    (`PrimitiveComponent.SetMaterial` (`self.StaticMesh`) _array_index _returnvalue)
    (`KismetArrayLibrary.Array_Add` (`self.Materials`) _returnvalue)))

(event `/Game/Input/Interface/BPI_Photoreactive.Burn`
  (bind _barrier (`self.Barrier`)
    (:`then`
      ; Activates dissolve effect, destroys actor
      (`self.K2_DestroyActor` _barrier))
    (:`else`
      _))
  (`PrimitiveComponent.SetCollisionEnabled` (`self.StaticMesh`) "NoCollision")
  (`AudioComponent.FadeIn` (`self.SC_Burn`) 0.1 1.0 0.0 "Linear")
  (bind (_direction _dissolve) (`Timeline|Timeline`)
    (:`Update`
      (for _array_element (`self.Materials`)
        (`MaterialInstanceDynamic.SetScalarParameterValue` _array_element "Dissolve" _dissolve)))
    (:`Finished`
      (bind _bellref (`self.BellRef`)
        (:`then`
          (`/Game/Prefabs/BP_Josiah/BP_Bell.FreeBell` _bellref))
        (:`else`
          _))
      (`self.K2_DestroyActor`))))

(fn `UserConstructionScript`)