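; Door for the Room 12 bell puzzle that opens once three bells are rung in order.
; Bell events advance a step counter; out-of-order second or third rings are ignored, while the first bell always resets it to one.
; The third step runs a timeline that moves the door's relative Z.
; Its update triggers a one-time level sequence, disabling BP_Ling's input for the duration.
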(event `self.ReceiveBeginPlay`
  (bind (_returnvalue_x _returnvalue_y _returnvalue_z) (`KismetMathLibrary.BreakVector` (`SceneComponent.K2_GetComponentLocation` (`self.Door`))))
  ; Find height
  (set `self.Return Value Z` _returnvalue_z))

(event `BellRung_1`
  ; Bell Order
  (set `self.BellOrder` 1))

(event `BellRung_2`
  ; Bell Order
  (if (== (`self.BellOrder`) 1)
    (set `self.BellOrder` 2)))

(event `OpenDoor`
  (bind _door (`self.Door`))
  (bind (_relativelocation_x _relativelocation_y) (`KismetMathLibrary.BreakVector` (`SceneComponent.RelativeLocation` _door)))
  ; Open/Close animation
  (bind (_direction _doorposition) (`Timeline|DoorActivation`)
    (:`Update`
      (`SceneComponent.K2_SetRelativeLocation` _door (`KismetMathLibrary.MakeVector` _relativelocation_x _relativelocation_y _doorposition) false false)
      (`self.PlaySequence`))))

(event `BellRung_3`
  ; Bell Order
  (if (== (`self.BellOrder`) 2)
    (set `self.BellOrder` 3)
    (`self.PuzzleFinished`)))

(event `PuzzleFinished`
  ; Bell Order
  (`self.OpenDoor`))

(event `PlaySequence`
  ; Play Sequence
  (`/Engine/EditorBlueprintResources/StandardMacros.DoOnce` false
    (:`Completed`
      (bind _outactor (`LevelSequencePlayer.CreateLevelSequencePlayer` "/Game/Sequences/LS_Room12Door.LS_Room12Door"))
      (bind _asbp_ling (cast `/Game/ThirdPerson/Blueprints/BP_Ling` (`GameplayStatics.GetPlayerCharacter` 0)))
      (`self.DisableInput` _asbp_ling null)
      (bind _sequenceplayer (`LevelSequenceActor.SequencePlayer` _outactor))
      (`MovieSceneSequencePlayer.Play` _sequenceplayer)
      (`KismetSystemLibrary.Delay` (`TimeManagementBlueprintLibrary.Conv_QualifiedFrameTimeToSeconds` (`MovieSceneSequencePlayer.GetDuration` _sequenceplayer)))
      (`self.EnableInput` _asbp_ling null))))

(fn `UserConstructionScript`)