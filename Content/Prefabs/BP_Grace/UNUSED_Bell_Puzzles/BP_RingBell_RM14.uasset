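; Puzzle bell actor that, when hit, rings one of three notes and reports it to a linked door.
; BeginPlay snaps the bell mesh onto its hinge component.
; Hit calls Ring and plays a timeline that swings the mesh on its roll axis.
; Ring branches on BellNote to call the matching BellRung event on DoorToActivate, add an audio component and print a debug number.
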(event `Ring`
  (bind _door_to_activate (`self.Door to Activate`))
  ; Plays when a bell is attached and hit by a projectile
  (set `self.BellNote` (`self.BellNote`))
  (if (== (`self.BellNote`) 0)
    (`KismetSystemLibrary.PrintString` "1")
    (`/Game/Prefabs/BP_Grace/UNUSED_Bell_Puzzles/BP_Door_BellPuzzle_RM12.BellRung_1` _door_to_activate)
    (`AddComponent|NODE_AddAudioComponent-1`)
    (elif (== (`self.BellNote`) 1)
      (`KismetSystemLibrary.PrintString` "2")
      (`/Game/Prefabs/BP_Grace/UNUSED_Bell_Puzzles/BP_Door_BellPuzzle_RM12.BellRung_2` _door_to_activate)
      (`AddComponent|NODE_AddAudioComponent-2`)
      (elif (== (`self.BellNote`) 2)
        (`KismetSystemLibrary.PrintString` "3")
        (`/Game/Prefabs/BP_Grace/UNUSED_Bell_Puzzles/BP_Door_BellPuzzle_RM12.BellRung_3` _door_to_activate)
        (`AddComponent|NODE_AddAudioComponent-3`)))))

(event `self.ReceiveHit`
  (params (MyComp :type "PrimitiveComponent Object Reference") (Other :type "Actor Object Reference") (OtherComp :type "PrimitiveComponent Object Reference") (bSelfMoved :type Boolean) (HitLocation :type "Vector Structure") (HitNormal :type "Vector Structure") (NormalImpulse :type "Vector Structure") (Hit :type "HitResult Structure (by ref)"))
  (bind _sm_bell (`self.SM_Bell`))
  (bind (_relativerotation_roll _relativerotation_pitch _relativerotation_yaw) (`KismetMathLibrary.BreakRotator` (`SceneComponent.RelativeRotation` _sm_bell)))
  ; Rings if attached to socket
  (`self.Ring`)
  (bind (_direction _ring_bell) (`Timeline|Timeline` :!via `PlayFromStart`)
    (:`Update`
      (`SceneComponent.K2_SetRelativeRotation` _sm_bell (`KismetMathLibrary.MakeRotator` _ring_bell _relativerotation_pitch _relativerotation_yaw) false false))))

(event `self.ReceiveBeginPlay`
  ; Attaches bell to socket
  (`SceneComponent.K2_AttachToComponent` (`self.SM_Bell`) (`self.Hinge`) "None" "SnapToTarget" "SnapToTarget" "KeepWorld" true))

(fn `UserConstructionScript`)