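; BP_LionStatue_RM8 is a lion statue, filed under unused bell puzzles, that plays a sound sequence when an actor approaches.
; Beginning overlap, with no filter on the actor, reveals a TextRender and calls SoundOrder; ending overlap hides the text.
; SoundOrder adds three audio components in turn, spaced by short fixed delays, and end overlap does not interrupt the sequence.
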(event `self.ReceiveActorBeginOverlap`
  (params (OtherActor :type "Actor Object Reference"))
  (`SceneComponent.SetVisibility` (`self.TextRender`) true false)
  (`self.SoundOrder`))

(event `self.ReceiveActorEndOverlap`
  (params (OtherActor :type "Actor Object Reference"))
  (`SceneComponent.SetVisibility` (`self.TextRender`) false false))

(event `SoundOrder`
  (`AddComponent|NODE_AddAudioComponent-0`)
  (`KismetSystemLibrary.Delay` 0.7)
  (`AddComponent|NODE_AddAudioComponent-1`)
  (`KismetSystemLibrary.Delay` 0.7)
  (`AddComponent|NODE_AddAudioComponent-2`))

(fn `UserConstructionScript`)