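; BP_HangingLantern is a hanging lantern prop whose point light can be shown or hidden during play.
; On BeginPlay, the Glowing setting decides whether the light starts visible.
; Trigger alternates the light through a FlipFlop that always shows it first, independent of Glowing.
; LightUp and LightDown events explicitly show or hide the light.
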(event `self.ReceiveBeginPlay`
  (bind _pointlight (`self.PointLight`))
  ; Sets light based on setting
  (if (`self.Glowing`)
    (`SceneComponent.SetHiddenInGame` _pointlight false false)
    (else
      (`SceneComponent.SetHiddenInGame` _pointlight true false))))

(event `LightUp`
  (`SceneComponent.SetHiddenInGame` (`self.PointLight`) false false))

(event `self.Trigger`
  (bind _pointlight (`self.PointLight`))
  ; Light up on hit
  (`/Engine/EditorBlueprintResources/StandardMacros.FlipFlop`
    (:`A`
      (`SceneComponent.SetHiddenInGame` _pointlight false false))
    (:`B`
      (`SceneComponent.SetHiddenInGame` _pointlight true false))))

(event `LightDown`
  (`SceneComponent.SetHiddenInGame` (`self.PointLight`) true false))

(fn `UserConstructionScript`)