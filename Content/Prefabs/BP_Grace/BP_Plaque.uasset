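; Plaque prop Blueprint that displays one of six symbols: butterfly, circle, dragon, moon, star or sun.
; On BeginPlay it switches on the SymbolType variable and sets the matching material instance on the first slot of the Plaque component.
; The construction script is empty, so the symbol is applied only when play starts.
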(event `self.ReceiveBeginPlay`
  (switch `int` (`self.SymbolType`)
    (:`1`
      ; Butterfly
      (`PrimitiveComponent.SetMaterial` (`self.Plaque`) 0 "/Game/Materials/VFX_Materials/Symbols/Plaque_Mats/MI_Plaque_Butterfly.MI_Plaque_Butterfly"))
    (:`2`
      ; Circle
      (`PrimitiveComponent.SetMaterial` (`self.Plaque`) 0 "/Game/Materials/VFX_Materials/Symbols/Plaque_Mats/MI_Plaque_Circle.MI_Plaque_Circle"))
    (:`3`
      ; Dragon
      (`PrimitiveComponent.SetMaterial` (`self.Plaque`) 0 "/Game/Materials/VFX_Materials/Symbols/Plaque_Mats/MI_Plaque_Dragon.MI_Plaque_Dragon"))
    (:`4`
      ; Moon
      (`PrimitiveComponent.SetMaterial` (`self.Plaque`) 0 "/Game/Materials/VFX_Materials/Symbols/Plaque_Mats/MI_Plaque_Moon.MI_Plaque_Moon"))
    (:`5`
      ; Star
      (`PrimitiveComponent.SetMaterial` (`self.Plaque`) 0 "/Game/Materials/VFX_Materials/Symbols/Plaque_Mats/MI_Plaque_Star.MI_Plaque_Star"))
    (:`6`
      ; Sun
      (`PrimitiveComponent.SetMaterial` (`self.Plaque`) 0 "/Game/Materials/VFX_Materials/Symbols/Plaque_Mats/MI_Plaque_Sun.MI_Plaque_Sun"))))

(fn `UserConstructionScript`)