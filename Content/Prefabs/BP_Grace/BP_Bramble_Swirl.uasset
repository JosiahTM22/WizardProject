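; BP_Bramble_Swirl is a vine obstacle actor that burns away when an illuminated BP_Ling enters its trigger.
; BeginPlay replaces every static mesh material with a dynamic instance stored in an array.
; The trigger checks Illuminated only on begin overlap and calls BurnVines, which waits briefly, adds audio, then drives each material's Dissolve parameter by timeline before destroying the actor.
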(event `self.ReceiveBeginPlay`
  ; Dissolve VFX, dissolves each material on actor
  (for (_array_element _array_index) (`MeshComponent.GetMaterials` (`self.StaticMesh`))
    ;; Dissolves both materials
    (bind _returnvalue (`KismetMaterialLibrary.CreateDynamicMaterialInstance` _array_element))
    (`PrimitiveComponent.SetMaterial` (`self.StaticMesh`) _array_index _returnvalue)
    (`KismetArrayLibrary.Array_Add` (`self.Materials`) _returnvalue)))

(event `BurnVines`
  ; Activates dissolve effect, destroys actor
  (`KismetSystemLibrary.Delay` 1.0)
  (`AddComponent|NODE_AddAudioComponent-0`)
  (bind (_direction _dissolve) (`Timeline|Timeline`)
    (:`Update`
      (for _array_element (`self.Materials`)
        (`MaterialInstanceDynamic.SetScalarParameterValue` _array_element "Dissolve" _dissolve)))
    (:`Finished`
      (`self.K2_DestroyActor`))))

(event `self.Trigger.OnComponentBeginOverlap`
  (params (OverlappedComponent :type "PrimitiveComponent Object Reference") (OtherActor :type "Actor Object Reference") (OtherComp :type "PrimitiveComponent Object Reference") (OtherBodyIndex :type Integer) (bFromSweep :type Boolean) (SweepResult :type "HitResult Structure (by ref)"))
  ; Burn activated upon overlap and IA_Input Illumination
  (bind _asbp_ling (cast `/Game/ThirdPerson/Blueprints/BP_Ling` OtherActor))
  (if (`/Game/ThirdPerson/Blueprints/BP_Ling.Illuminated` _asbp_ling)
    (`self.BurnVines`)
    (else
      (set `/Game/ThirdPerson/Blueprints/BP_Ling.Illuminated` false _asbp_ling))))

(fn `UserConstructionScript`)