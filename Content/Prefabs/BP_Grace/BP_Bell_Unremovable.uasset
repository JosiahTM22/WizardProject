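; BP_Bell_Unremovable is a bell that starts attached to a linked BellSocket and rings when triggered.
; On BeginPlay it snaps its mesh to the socket's attach point and notifies the socket.
; Trigger rings the socket and toggles a Floating flag with an overlay material, playing a timeline that rolls the mesh only when Floating turns on.
; Without a valid socket, Trigger just prints "Thunk".
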(event `self.Trigger`
  (bind _sm_bell (`self.SM_Bell`))
  (bind _sm_bell_2 (`self.SM_Bell`))
  (bind (_relativerotation_roll _relativerotation_pitch _relativerotation_yaw) (`KismetMathLibrary.BreakRotator` (`SceneComponent.RelativeRotation` _sm_bell_2)))
  ; Rings if attached to socket -- attached by default (link it with the eyedropper)
  (bind _bellsocket (`self.BellSocket`)
    (:`then`
      (`/Game/Prefabs/BP_Grace/BP_Socket_Unremovable.Ring` _bellsocket)
      (if (`self.Floating`)
        (`MeshComponent.SetOverlayMaterial` _sm_bell null)
        (set `self.Floating` false)
        (else
          (`MeshComponent.SetOverlayMaterial` _sm_bell "/Game/Materials/Mat_Overlay.Mat_Overlay")
          (set `self.Floating` true)
          (bind (_direction _ring_bell) (`Timeline|Ring Bell` :!via `PlayFromStart`)
            (:`Update`
              (`SceneComponent.K2_SetRelativeRotation` _sm_bell_2 (`KismetMathLibrary.MakeRotator` _ring_bell _relativerotation_pitch _relativerotation_yaw) false false))))))
    (:`else`
      (`KismetSystemLibrary.PrintString` "Thunk"))))

(event `self.ReceiveBeginPlay`
  ; Attaches if default
  (bind _bellsocket (`self.BellSocket`)
    (:`then`
      (`SceneComponent.K2_AttachToComponent` (`self.SM_Bell`) (`/Game/Prefabs/BP_Grace/BP_Socket_Unremovable.AttachPoint` _bellsocket) "None" "SnapToTarget" "SnapToTarget" "KeepWorld" true)
      (`/Game/Prefabs/BP_Grace/BP_Socket_Unremovable.AttachBell` _bellsocket))
    (:`else`)))

(fn `UserConstructionScript`)