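; A switch-driven door that opens when enough switches are active and closes when the count drops below the required number.
; Switch activated and deactivated events adjust a counter, skipping inputs above a Zero threshold, then share one check against SwitchesNeeded.
; The DoorActivation timeline plays or reverses to set the door's relative Z position.
; With OneTimeOpen set, the door latches open and ignores later count changes.
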(event `self.ReceiveBeginPlay`
  (bind (_returnvalue_x _returnvalue_y _returnvalue_z) (`KismetMathLibrary.BreakVector` (`SceneComponent.K2_GetComponentLocation` (`self.Door`))))
  ; Find height
  (set `self.Return Value Z` _returnvalue_z))

(event `SwitchActivated`
  (params (OpenNum :type Integer))
  (bind _door (`self.Door`))
  (bind (_relativelocation_x _relativelocation_y) (`KismetMathLibrary.BreakVector` (`SceneComponent.RelativeLocation` _door)))
  (if (not (> OpenNum (`self.Zero`)))
    ; Opens and closes door based on the number of activated switches
    (`/Engine/EditorBlueprintResources/StandardMacros.IncrementInt` (`self.SwitchesActive`)
      (:`  `
        (if (`self.Opened`) :!label _label
          _
          (elif (>= (`self.SwitchesActive`) (`self.SwitchesNeeded`))
            ; Checks if the door opens permanently
            (if (`self.OneTimeOpen`)
              (set `self.Opened` true)
              ; Open/Close animation
              (bind (_direction _doorposition) (`Timeline|DoorActivation` :!label _label_2)
                (:`Update`
                  (`SceneComponent.K2_SetRelativeLocation` _door (`KismetMathLibrary.MakeVector` _relativelocation_x _relativelocation_y _doorposition) false false)))
              (else
                (goto _label_2)))
            (else
              (goto _label_2 :!via `Reverse`))))))))

(event `SwitchDeactivated`
  (params (CloseNum :type Integer))
  (if (not (> CloseNum (`self.Zero`)))
    ; Opens and closes door based on the number of activated switches
    (`/Engine/EditorBlueprintResources/StandardMacros.DecrementInt` (`self.SwitchesActive`)
      (:`  `
        (goto _label)))))

(fn `UserConstructionScript`)