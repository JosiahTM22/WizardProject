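; BP_BellPuzzle is a puzzle actor that checks whether bells are triggered in a correct order.
; On BeginPlay it finds every BP_Bell in the level and hands each a reference to itself.
; RegisterBellInput compares an index to the current step of CorrectSequence, advancing on a match and resetting to zero on a mismatch.
; Completing the sequence only prints "Door Opened"; no door logic exists here.
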(event `self.ReceiveBeginPlay`
  (bind _outactors (`GameplayStatics.GetAllActorsOfClass` "/Game/BluePrint/BP_Bell.BP_Bell_C"))
  (for _array_element _outactors
    (set `/Game/BluePrint/BP_Bell.PuzzleRef` self _array_element)))

(fn `RegisterBellInput`
  (params (InputIndex :type Integer))
  (if (== InputIndex (`|GetArrayItem` (`self.CorrectSequence`) (`self.CurrentStep`)))
    (set `self.CurrentStep` (+ (`self.CurrentStep`) 1))
    (if (== (`self.CurrentStep`) (`KismetArrayLibrary.Array_Length` (`self.CorrectSequence`)))
      (`KismetSystemLibrary.PrintString` "Door Opened"))
    (else
      (set `self.CurrentStep` 0)
      (`KismetSystemLibrary.PrintString` "Wrong order"))))

(fn `UserConstructionScript`)