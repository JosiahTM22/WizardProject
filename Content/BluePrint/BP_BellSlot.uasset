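; BP_BellSlot is a puzzle slot that checks whether the BP_Bell placed in its SlotTrigger matches its SlotIndex.
; BeginPlay checks bells already overlapping and marks matches as placed correctly.
; Begin overlap sets each bell's IsPlacedCorrectly from the index comparison and end overlap resets it, with debug prints on entry.
; AssignedSlot is only ever written as None, so the slot never registers itself on the bell.
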(event `self.ReceiveBeginPlay`
  (for _array_element (`PrimitiveComponent.GetOverlappingActors` (`self.SlotTrigger`) null)
    (bind _asbp_bell (cast `/Game/BluePrint/BP_Bell` _array_element))
    (if (== (`self.SlotIndex`) (`/Game/BluePrint/BP_Bell.BellIndex` _asbp_bell))
      (set `/Game/BluePrint/BP_Bell.IsPlacedCorrectly` true _asbp_bell)
      (set `/Game/BluePrint/BP_Bell.AssignedSlot` null _asbp_bell)
      (else
        (`KismetSystemLibrary.PrintString` "Begin Play Wrong SLot")))))

(event `self.SlotTrigger.OnComponentBeginOverlap`
  (params (OverlappedComponent :type "PrimitiveComponent Object Reference") (OtherActor :type "Actor Object Reference") (OtherComp :type "PrimitiveComponent Object Reference") (OtherBodyIndex :type Integer) (bFromSweep :type Boolean) (SweepResult :type "HitResult Structure (by ref)"))
  (bind _asbp_bell (cast `/Game/BluePrint/BP_Bell` OtherActor)
    (:`then`
      (if (== (`self.SlotIndex`) (`/Game/BluePrint/BP_Bell.BellIndex` _asbp_bell))
        (`KismetSystemLibrary.PrintString` "Correct Slot")
        (set `/Game/BluePrint/BP_Bell.IsPlacedCorrectly` true _asbp_bell)
        (set `/Game/BluePrint/BP_Bell.AssignedSlot` null _asbp_bell)
        (else
          (`KismetSystemLibrary.PrintString` "Wrong Slot")
          (set `/Game/BluePrint/BP_Bell.IsPlacedCorrectly` false _asbp_bell)
          (set `/Game/BluePrint/BP_Bell.AssignedSlot` null _asbp_bell))))
    (:`CastFailed`
      (`KismetSystemLibrary.PrintString` "Slot Cast Failed"))))

(event `self.SlotTrigger.OnComponentEndOverlap`
  (params (OverlappedComponent :type "PrimitiveComponent Object Reference") (OtherActor :type "Actor Object Reference") (OtherComp :type "PrimitiveComponent Object Reference") (OtherBodyIndex :type Integer))
  (bind _asbp_bell (cast `/Game/BluePrint/BP_Bell` OtherActor))
  (set `/Game/BluePrint/BP_Bell.IsPlacedCorrectly` false _asbp_bell)
  (set `/Game/BluePrint/BP_Bell.AssignedSlot` null _asbp_bell))

(fn `UserConstructionScript`)